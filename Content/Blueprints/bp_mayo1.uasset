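; bp_mayo1 is a mayo item actor that the third-person character can pick up and use.
; On overlap it caches the character and calls its TrytopickupITEM with itself.
; Pickup plays a sound and attaches it to the character mesh's left middle-finger socket.
; Drop plays a sound and destroys it, while PrimaryAction spawns another Bp_mayo1 at its current transform.
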(event `self.ReceiveActorBeginOverlap`
  (params (OtherActor :type "Actor Object Reference"))
  (bind _asbp_third_person_character (cast `/Game/ThirdPerson/Blueprints/BP_ThirdPersonCharacter` OtherActor))
  (set `self.bp_thirdperson` _asbp_third_person_character)
  (`/Game/ThirdPerson/Blueprints/BP_ThirdPersonCharacter.trytopickupITEM` _asbp_third_person_character self))

(event `/Game/Blueprints/BPI_item.pickup`
  (`GameplayStatics.PlaySound2D` "/Engine/VREditor/Sounds/UI/Object_PickUp.Object_PickUp" 1.0 1.0 0.0 null null)
  (`self.K2_AttachToComponent` (`Character.Mesh` (`self.bp_thirdperson`)) "middle_01_l" "SnapToTarget" "SnapToTarget" "KeepRelative"))

(event `/Game/Blueprints/BPI_item.drop`
  (`GameplayStatics.PlaySound2D` "/Engine/EngineSounds/WhiteNoise.WhiteNoise" 1.0 1.0 0.0 null null)
  (`self.K2_DestroyActor`))

(event `/Game/Blueprints/BPI_item.primary action`
  (`|SpawnActorFromClass` "bp_mayo1_C" (`self.GetTransform`) "Undefined" "MultiplyWithRoot" null null))

(fn `UserConstructionScript`)