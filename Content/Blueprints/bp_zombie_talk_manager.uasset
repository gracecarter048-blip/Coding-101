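; Dialogue manager for zombie talk that shows the next line from its dialogue array each time DisplayNextLine fires.
; BeginPlay creates a W_dialogue widget, which each call fills with the current line, adds to the viewport and removes after a ten-second delay, alongside a printed copy.
; The index advances without waiting for that delay, and calls past the last line do nothing because the index reset is unconnected.
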(event `self.ReceiveBeginPlay`
  (bind _returnvalue (`|CreateWidget` "/Game/widgets/W_dialogue.W_dialogue_C"))
  (set `self.dialoge_widget` _returnvalue))

(event `Display Next Line`
  (bind _dialoge_widget (`self.dialoge_widget`))
  (bind _output (`|GetArrayItem` (`self.dialoge`) (`self.index`)))
  (if (not (>= (`self.index`) (`KismetArrayLibrary.Array_Length` (`self.dialoge`))))
    (`KismetSystemLibrary.PrintText` _output true true (struct :`R` 1.0 :`G` 0.841834 :`A` 1.0) 30.0)
    (`TextBlock.SetText` (`/Game/widgets/W_dialogue.TextBlock_0` (`self.dialoge_widget`)) _output)
    (`|ExecutionSequence`
      (:`then_0`
        (`UserWidget.AddToViewport` _dialoge_widget 0)
        (`KismetSystemLibrary.Delay` 10.0)
        (`Widget.RemoveFromParent` _dialoge_widget))
      (:`then_1`
        (`/Engine/EditorBlueprintResources/StandardMacros.IncrementInt` (`self.index`))))))

(fn `UserConstructionScript`)