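; Tree plantation actor that has the third-person player character plant a tree, then removes itself.
; Player overlap and the T key both run PlantTree on the character cast from the overlap, with no check that T was pressed.
; An always-true branch then unhides a coin icon mesh, prints congratulations and destroys the actor.
; A separate custom event, not called here, increments the player's TotalKeys and destroys the actor.
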(event `Key|T`
  (params (Key :type "Key Structure"))
  (:`Pressed`
    (`/Game/ThirdPerson/Blueprints/BP_ThirdPersonCharacter.plant tree` (stale `self.ReceiveActorBeginOverlap` _asbp_third_person_character) :!label _label)
    (if true
      (`SceneComponent.SetHiddenInGame` (`self.SM_PolygonPrototype_Icon_Coin_01`) false false)
      (`KismetSystemLibrary.PrintString` "Congratulations for growing the forest!" true true (struct :`R` 0.22914 :`G` 0.894792 :`B` 0.053128 :`A` 1.0) 16.0)
      (`self.K2_DestroyActor`))))

(event `self.ReceiveActorBeginOverlap`
  (params (OtherActor :type "Actor Object Reference"))
  (bind _asbp_third_person_character (cast `/Game/ThirdPerson/Blueprints/BP_ThirdPersonCharacter` OtherActor))
  (goto _label))

(event `CustomEvent`
  (params (OtherActor :type "Actor Object Reference"))
  (bind _asbp_third_person_character (cast `/Game/ThirdPerson/Blueprints/BP_ThirdPersonCharacter` OtherActor)) ; was it the player that hit us?
  (`/Engine/EditorBlueprintResources/StandardMacros.IncrementInt` (`/Game/ThirdPerson/Blueprints/BP_ThirdPersonCharacter.total keys` _asbp_third_person_character) ; add 1 to total keys on the player
    (:`  `
      (`self.K2_DestroyActor`))))

(fn `UserConstructionScript`)