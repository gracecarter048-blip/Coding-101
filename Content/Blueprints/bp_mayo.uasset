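; bp_mayo is an actor that slides a mayo mesh between Start and End points.
; On BeginPlay it plays a half-volume, half-pitch movement sound and starts a timeline that lerps the mesh's relative location between the two points.
; Each timeline update wires back into the sound and Play calls, so the sound fires again on every update.
; The sound's location comes from Start's relative, not world, position.
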(event `self.ReceiveBeginPlay`
  (`GameplayStatics.PlaySoundAtLocation` "/Engine/VREditor/Sounds/VR_WorldMoveLoop_02.VR_WorldMoveLoop_02" (`SceneComponent.RelativeLocation` (`self.start`)) (struct) 0.5 0.5 0.0 null null null null :!label _label)
  (bind (_direction _newtrack_0) (`Timeline|Timeline`)
    (:`Update`
      (`SceneComponent.K2_SetRelativeLocation` (`self.mayoglb`) (`KismetMathLibrary.VLerp` (`SceneComponent.RelativeLocation` (`self.start`)) (`SceneComponent.RelativeLocation` (`self.end`)) _newtrack_0) false false)
      (goto _label))))

(fn `UserConstructionScript`)