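; A locked door Blueprint that opens when the third-person player character overlaps it while holding at least one key.
; On overlap it plays a sound and prints a knocking message, then checks the character's TotalKeys count.
; With a key, it spends one and destroys the door mesh and overlap box, so the door stays open; otherwise it prints that it is locked.
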(event `self.ReceiveActorBeginOverlap`
  (params (OtherActor :type "Actor Object Reference"))
  (bind _asbp_third_person_character (cast `/Game/ThirdPerson/Blueprints/BP_ThirdPersonCharacter` OtherActor))
  (`GameplayStatics.PlaySound2D` "/Engine/VREditor/Sounds/VR_grab_Cue.VR_grab_Cue" 1.0 1.0 0.0 null null)
  (`KismetSystemLibrary.PrintText` "Player is knocking")
  (bind _total_keys (`/Game/ThirdPerson/Blueprints/BP_ThirdPersonCharacter.total keys` _asbp_third_person_character))
  (if (> _total_keys 0)
    (`/Engine/EditorBlueprintResources/StandardMacros.DecrementInt` _total_keys
      (:`  `
        (`ActorComponent.K2_DestroyComponent` (`self.SM_Bld_Door_01`))
        (`ActorComponent.K2_DestroyComponent` (`self.overlap box`))))
    (else
      (`KismetSystemLibrary.PrintText` "It is locked"))))

(fn `UserConstructionScript`)