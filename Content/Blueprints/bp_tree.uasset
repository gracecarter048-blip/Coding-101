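; Tree Blueprint that picks a random mesh on BeginPlay and grows in randomized steps.
; A DoN-gated loop waits a random few seconds, then adds a random amount to the mesh's relative scale.
; After each step it compares the DoN counter to a random integer, enabling query and physics collision on a match and otherwise looping through the randomly limited gate again.
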(event `self.ReceiveBeginPlay`
  (`StaticMeshComponent.SetStaticMesh` (`self.tree`) (`KismetArrayLibrary.Array_Random` (`self.New Mesh`)))
  (`self.growloop`))

(event `growloop`
  (bind _returnvalue (`KismetMathLibrary.RandomIntegerInRange` 1 5))
  (bind _counter (`/Engine/EditorBlueprintResources/StandardMacros.Do N` _returnvalue :!label _label)
    (:`Exit`
      (`KismetSystemLibrary.Delay` (`KismetMathLibrary.RandomFloatInRange` 3.0 5.0))
      (`self.grow`)
      (if (== _counter _returnvalue)
        (`PrimitiveComponent.SetCollisionEnabled` (`self.tree`) "QueryAndPhysics")
        (`KismetSystemLibrary.PrintText` "Hellocollision enabled")
        (else
          (goto _label))))))

(event `grow`
  (bind _tree (`self.tree`))
  (set `self.colors` (`self.colors`))
  (`SceneComponent.SetRelativeScale3D` _tree (+ (`SceneComponent.RelativeScale3D` _tree) (`KismetMathLibrary.RandomFloatInRange` 0.2 0.4))))

(fn `UserConstructionScript`)