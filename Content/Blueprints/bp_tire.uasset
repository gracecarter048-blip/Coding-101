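; Tire actor that spins while its car wheel mesh slides between two points, with no overlap or other gameplay logic.
; On BeginPlay, a timeline drives a lerp of the mesh's relative location from the Start component to the End component, without sweeping.
; Tick adds local yaw to the whole actor at the Rotation rate scaled by delta time, so the slide path turns with it.
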(event `self.ReceiveBeginPlay`
  (bind (_direction _newtrack_0) (`Timeline|Timeline`)
    (:`Update`
      (`SceneComponent.K2_SetRelativeLocation` (`self.SM_PolygonCity_Veh_Car_Small_Wheel_fl`) (`KismetMathLibrary.VLerp` (`SceneComponent.RelativeLocation` (`self.start`)) (`SceneComponent.RelativeLocation` (`self.end`)) _newtrack_0) false false))))

(event `self.ReceiveTick`
  (params (DeltaSeconds :type "Float (single-precision)"))
  (`self.K2_AddActorLocalRotation` (`KismetMathLibrary.MakeRotator` 0.0 0.0 (* (`self.rotation`) DeltaSeconds))))

(fn `UserConstructionScript`)