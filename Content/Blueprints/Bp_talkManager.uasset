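; Dialogue manager Blueprint that shows lines from a Dialogue array one at a time on screen.
; It creates a W_dialogue widget at BeginPlay, and each DisplayNextLine call prints the current line, sets the widget's text and shows it briefly before a delayed removal.
; The index advances immediately, and calls past the last line do nothing because the index reset is left unconnected.
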(event `self.ReceiveBeginPlay`
  (bind _returnvalue (`|CreateWidget` "/Game/widgets/W_dialogue.W_dialogue_C"))
  (set `self.dialogue-widget` _returnvalue))

(event `Display Next Line`
  (bind _dialogue_widget (`self.dialogue-widget`))
  (bind _output (`|GetArrayItem` (`self.dialogue`) (`self.index`)))
  (if (not (>= (`self.index`) (`KismetArrayLibrary.Array_Length` (`self.dialogue`))))
    (`KismetSystemLibrary.PrintText` _output true true (struct :`R` 1.0 :`G` 0.841834 :`A` 1.0) 30.0)
    (`TextBlock.SetText` (`/Game/widgets/W_dialogue.TextBlock_0` (`self.dialogue-widget`)) _output)
    (`|ExecutionSequence`
      (:`then_0`
        (`UserWidget.AddToViewport` _dialogue_widget 0)
        (`KismetSystemLibrary.Delay` 10.0)
        (`Widget.RemoveFromParent` _dialogue_widget))
      (:`then_1`
        (`/Engine/EditorBlueprintResources/StandardMacros.IncrementInt` (`self.index`))))))

(fn `UserConstructionScript`)