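; Demo Blueprint for loop and array techniques, using debug prints and Bp_tree actors in the level.
; BeginPlay starts a Delay-driven repeating loop and a while countdown that prints color-cycled messages.
; Each repeat calls an event that shuffles all trees and gives them random yaw one at a time, using an index and short Delay.
; An uncalled for-each event sets every tree's rotation at once, with its random range set to zero.
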(event `self.ReceiveBeginPlay`
  (`KismetSystemLibrary.PrintText` "loops and lists starting")
  (`self.simple loop`)
  (`self.while loop function`))

(event `simple loop`
  (`KismetSystemLibrary.PrintText` "inside simple loop waiting 3 seconds" :!label _label)
  (`self.loopArrayOverTime`)
  (`KismetSystemLibrary.Delay` 3.0)
  (goto _label))

(event `while loop function`
  (bind _colors (`self.colors`))
  (while (> (`self.while counter`) 0)
    (`KismetSystemLibrary.PrintText` (`|FormatText` "this is loop{count} ran after {seconds} seconds" (`self.while counter`) (`KismetTextLibrary.Conv_DoubleToText` (`GameplayStatics.GetRealTimeSeconds`) "HalfToEven" false true 1 100)) true true (`|GetArrayItem` _colors (mod (`self.while counter`) (`KismetArrayLibrary.Array_Length` _colors))) 20.0)
    (`/Engine/EditorBlueprintResources/StandardMacros.DecrementInt` (`self.while counter`))))

(event `change-treesFor each loop`
  (bind _outactors (`GameplayStatics.GetAllActorsOfClass` "/Game/Blueprints/bp_tree.bp_tree_C"))
  (for _array_element _outactors
    (`self.K2_SetActorRelativeRotation` _array_element (`KismetMathLibrary.MakeRotator` 0.0 0.0 (`KismetMathLibrary.RandomFloatInRange` 0.0)) false false)))

(event `loopArrayOverTime`
  (bind _outactors (`GameplayStatics.GetAllActorsOfClass` "/Game/Blueprints/bp_tree.bp_tree_C"))
  (`KismetArrayLibrary.Array_Shuffle` _outactors)
  (if (< (`self.overtimeIndex`) (`KismetArrayLibrary.Array_Length` _outactors)) :!label _label_2
    (`self.K2_SetActorRelativeRotation` (`|GetArrayItem` _outactors (`self.overtimeIndex`)) (`KismetMathLibrary.MakeRotator` 0.0 0.0 (`KismetMathLibrary.RandomFloatInRange` 0.0 360.0)) false false)
    (`/Engine/EditorBlueprintResources/StandardMacros.IncrementInt` (`self.overtimeIndex`)
      (:`  `
        (`KismetSystemLibrary.Delay` 0.2)
        (goto _label_2)))
    (else
      (set `self.overtimeIndex` 0))))

(fn `UserConstructionScript`)