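; Locked gate door that the third-person character opens by spending a key.
; On actor overlap it plays a sound, then either decrements TotalKeys and destroys the OverlapBox, or prints that it is locked.
; A FlipFlop alternates playing and reversing the DoorAmin timeline, whose track scales ZRotation to yaw the Gate.
; OverlapBox begin and end overlaps both enable player input on the actor.
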(event `self.ReceiveActorBeginOverlap`
  (params (OtherActor :type "Actor Object Reference"))
  (bind _asbp_third_person_character (cast `/Game/ThirdPerson/Blueprints/BP_ThirdPersonCharacter` OtherActor))
  (`GameplayStatics.PlaySound2D` "/Engine/VREditor/Sounds/VR_grab_Cue.VR_grab_Cue" 1.0 1.0 0.0 null null)
  (bind _total_keys (`/Game/ThirdPerson/Blueprints/BP_ThirdPersonCharacter.total keys` _asbp_third_person_character))
  (if (> _total_keys 0)
    (`/Engine/EditorBlueprintResources/StandardMacros.DecrementInt` _total_keys
      (:`  `
        (`ActorComponent.K2_DestroyComponent` (`self.overlap box`))
        (`/Engine/EditorBlueprintResources/StandardMacros.FlipFlop`
          (:`A`
            (bind (_direction _newtrack_0) (`Timeline|door amin` :!label _label)
              (:`Update`
                (`SceneComponent.K2_SetRelativeRotation` (`self.Gate`) (`KismetMathLibrary.MakeRotator` 0.0 0.0 (* _newtrack_0 (`self.Z Rotation`))) false false))))
          (:`B`
            (goto _label :!via `Reverse`)))))
    (else
      (`KismetSystemLibrary.PrintText` "It is locked"))))

(event `self.overlap box.OnComponentBeginOverlap`
  (params (OverlappedComponent :type "PrimitiveComponent Object Reference") (OtherActor :type "Actor Object Reference") (OtherComp :type "PrimitiveComponent Object Reference") (OtherBodyIndex :type Integer) (bFromSweep :type Boolean) (SweepResult :type "HitResult Structure (by ref)"))
  (cast `/Game/ThirdPerson/Blueprints/BP_ThirdPersonCharacter` OtherActor)
  (`self.EnableInput` (`GameplayStatics.GetPlayerController` 0)))

(event `self.overlap box.OnComponentEndOverlap`
  (params (OverlappedComponent :type "PrimitiveComponent Object Reference") (OtherActor :type "Actor Object Reference") (OtherComp :type "PrimitiveComponent Object Reference") (OtherBodyIndex :type Integer))
  (cast `/Game/ThirdPerson/Blueprints/BP_ThirdPersonCharacter` OtherActor)
  (`self.EnableInput` (`GameplayStatics.GetPlayerController` 0)))

(fn `UserConstructionScript`)