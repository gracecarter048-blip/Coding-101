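; BP_rockSpawner is a "rock planter" item that the third-person character can pick up and use to spawn actors.
; On overlap it stores the character and offers itself through TrytopickupITEM.
; Pickup snaps it to the character mesh's HandGrip_L socket, and Drop destroys it.
; PrimaryAction spawns a Bp_key at its own transform, despite the rock naming and debug text.
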(event `self.ReceiveActorBeginOverlap`
  (params (OtherActor :type "Actor Object Reference"))
  (bind _asbp_third_person_character (cast `/Game/ThirdPerson/Blueprints/BP_ThirdPersonCharacter` OtherActor))
  (set `self.player` _asbp_third_person_character)
  (`/Game/ThirdPerson/Blueprints/BP_ThirdPersonCharacter.trytopickupITEM` _asbp_third_person_character self))

(event `/Game/Blueprints/BPI_item.pickup`
  (`KismetSystemLibrary.PrintText` "the rock planter is getting picked up!")
  (`self.K2_AttachToComponent` (`Character.Mesh` (`self.player`)) "HandGrip_L" "SnapToTarget" "SnapToTarget" "KeepRelative"))

(event `/Game/Blueprints/BPI_item.primary action`
  (`KismetSystemLibrary.PrintText` "Lets plant some rocks")
  (`|SpawnActorFromClass` "/Game/Blueprints/bp_key.bp_key_C" (`self.GetTransform`) "Undefined" "MultiplyWithRoot" null null))

(event `/Game/Blueprints/BPI_item.drop`
  (`KismetSystemLibrary.PrintText` "The rock planter is getting dropped")
  (`self.K2_DestroyActor`))

(fn `UserConstructionScript`)