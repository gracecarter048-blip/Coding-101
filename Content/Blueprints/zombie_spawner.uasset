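; Trigger-volume actor that spawns a group of zombies when the player walks into it.
; On BeginPlay it caches the player as BP_ThirdPersonCharacter, then the Box overlap checks against that reference and uses DoOnce so the ambush fires a single time.
; The spawn event creates one Zombie AI at the world location and rotation of each of three Billboard components, which serve as spawn points.
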(event `self.ReceiveBeginPlay`
  (bind _asbp_third_person_character (cast `/Game/ThirdPerson/Blueprints/BP_ThirdPersonCharacter` (`GameplayStatics.GetPlayerCharacter` 0)))
  (set `self.As BP Third Person Character` _asbp_third_person_character))

(event `self.Box.OnComponentBeginOverlap`
  (params (OverlappedComponent :type "PrimitiveComponent Object Reference") (OtherActor :type "Actor Object Reference") (OtherComp :type "PrimitiveComponent Object Reference") (OtherBodyIndex :type Integer) (bFromSweep :type Boolean) (SweepResult :type "HitResult Structure (by ref)"))
  (if (== OtherActor (`self.As BP Third Person Character`))
    (`/Engine/EditorBlueprintResources/StandardMacros.DoOnce` false
      (:`Completed`
        (`self.spawn zombie`)))))

(event `spawn zombie`
  (bind _billboard2 (`self.Billboard2`))
  (bind _billboard (`self.Billboard`))
  (bind _billboard1 (`self.Billboard1`))
  (`|ExecutionSequence`
    (:`then_0`
      (`AIBlueprintHelperLibrary.SpawnAIFromClass` "/Game/stuff/NewFolder/zombie.zombie_C" null (`SceneComponent.K2_GetComponentLocation` _billboard) (`SceneComponent.K2_GetComponentRotation` _billboard) false null))
    (:`then_1`
      (`AIBlueprintHelperLibrary.SpawnAIFromClass` "/Game/stuff/NewFolder/zombie.zombie_C" null (`SceneComponent.K2_GetComponentLocation` _billboard1) (`SceneComponent.K2_GetComponentRotation` _billboard1) false null))
    (:`then_2`
      (`AIBlueprintHelperLibrary.SpawnAIFromClass` "/Game/stuff/NewFolder/zombie.zombie_C" null (`SceneComponent.K2_GetComponentLocation` _billboard2) (`SceneComponent.K2_GetComponentRotation` _billboard2) false null))))

(fn `UserConstructionScript`)