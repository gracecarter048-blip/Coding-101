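; An axe item Blueprint (bp_ax) that the third-person character can pick up, use and drop.
; On overlap it caches the BP_ThirdPersonCharacter and passes itself to TrytopickupITEM, while its Pickup event snaps it to the middle_01_l socket on that character's mesh.
; PrimaryAction spawns a Bp_throw actor at the item's transform without removing the held item.
; Drop destroys the item outright.
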(event `self.ReceiveActorBeginOverlap`
  (params (OtherActor :type "Actor Object Reference"))
  (bind _asbp_third_person_character (cast `/Game/ThirdPerson/Blueprints/BP_ThirdPersonCharacter` OtherActor))
  (set `self.bp_thirdperson` _asbp_third_person_character)
  (`/Game/ThirdPerson/Blueprints/BP_ThirdPersonCharacter.trytopickupITEM` _asbp_third_person_character self))

(event `/Game/Blueprints/BPI_item.pickup`
  (`self.K2_AttachToComponent` (`Character.Mesh` (`self.bp_thirdperson`)) "middle_01_l" "SnapToTarget" "SnapToTarget" "KeepRelative"))

(event `/Game/Blueprints/BPI_item.primary action`
  (`|SpawnActorFromClass` "/Game/Blueprints/bp_throw.bp_throw_C" (`self.GetTransform`) "Undefined" "MultiplyWithRoot" null null))

(event `/Game/Blueprints/BPI_item.drop`
  (`self.K2_DestroyActor`))

(fn `UserConstructionScript`)