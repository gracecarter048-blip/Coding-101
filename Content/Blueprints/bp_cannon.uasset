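; Pickup cannon actor that offers itself to the third-person character on overlap and snaps to a socket on the character's mesh when picked up.
; Releasing Z fires after a short delay, spawning a Bp_throw projectile at SpawnPoint and applying a large forward force to it.
; PrimaryAction spawns the same projectile at the actor's transform without adding force, and Drop destroys the cannon.
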(event `Key|Z`
  (params (Key :type "Key Structure"))
  (:`Released`
    (`KismetSystemLibrary.Delay` 0.5)
    (`self.firecannon`)))

(event `firecannon`
  (bind _returnvalue (`|SpawnActorFromClass` "/Game/Blueprints/bp_throw.bp_throw_C" (`SceneComponent.K2_GetComponentToWorld` (`self.spawnPoint`)) "Undefined" "MultiplyWithRoot" null null))
  (`PrimitiveComponent.AddForce` (`/Game/Blueprints/bp_throw.Watergun_01_Refill` _returnvalue) (* (`SceneComponent.GetForwardVector` (`self.spawnPoint`)) 200000.0) "None" true))

(event `self.ReceiveActorBeginOverlap`
  (params (OtherActor :type "Actor Object Reference"))
  (bind _asbp_third_person_character (cast `/Game/ThirdPerson/Blueprints/BP_ThirdPersonCharacter` OtherActor))
  (set `self.bp third person` _asbp_third_person_character)
  (`/Game/ThirdPerson/Blueprints/BP_ThirdPersonCharacter.trytopickupITEM` _asbp_third_person_character self))

(event `/Game/Blueprints/BPI_item.pickup`
  (`self.K2_AttachToComponent` (`Character.Mesh` (`self.bp third person`)) "middle_01_l" "SnapToTarget" "SnapToTarget" "KeepRelative"))

(event `/Game/Blueprints/BPI_item.primary action`
  (`|SpawnActorFromClass` "/Game/Blueprints/bp_throw.bp_throw_C" (`self.GetTransform`) "Undefined" "MultiplyWithRoot" null null))

(event `/Game/Blueprints/BPI_item.drop`
  (`self.K2_DestroyActor`))

(fn `UserConstructionScript`)