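; Spike platform hazard that sends the player back to their checkpoint on contact.
; A timeline started at BeginPlay drives the local Z of the Spike9 component through a lerp, moving it like a vertical piston.
; When Spike9 begins overlapping a BP_ThirdPersonCharacter, it plays a 2D sound and calls ResetToCheckPoint on that character.
; A positional sound node is left unconnected.
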(event `self.ReceiveBeginPlay`
  (`|ExecutionSequence`
    (:`then_0`
      (bind (_direction _vertical_piston_location) (`Timeline|Timeline` :!via `SetNewTime` :!label _label)
        (:`Update`
          (`SceneComponent.K2_SetRelativeLocation` null (`KismetMathLibrary.MakeVector` 0.0 0.0 (`KismetMathLibrary.Lerp` 25.0 50.0 _vertical_piston_location)) false false)
          (`SceneComponent.K2_SetRelativeLocation` (`self.spike9`) (`KismetMathLibrary.MakeVector` 0.0 0.0 (`KismetMathLibrary.Lerp` 25.0 50.0 _vertical_piston_location)) false false)
          (goto _label))))
    (:`then_1`
      (goto _label))))

(event `self.spike9.OnComponentBeginOverlap`
  (params (OverlappedComponent :type "PrimitiveComponent Object Reference") (OtherActor :type "Actor Object Reference") (OtherComp :type "PrimitiveComponent Object Reference") (OtherBodyIndex :type Integer) (bFromSweep :type Boolean) (SweepResult :type "HitResult Structure (by ref)"))
  (bind _asbp_third_person_character (cast `/Game/ThirdPerson/Blueprints/BP_ThirdPersonCharacter` OtherActor))
  (`GameplayStatics.PlaySound2D` "/Engine/VREditor/Sounds/VR_close_Cue.VR_close_Cue" 1.0 1.0 0.0 null null)
  (`/Game/ThirdPerson/Blueprints/BP_ThirdPersonCharacter.reset to check point` _asbp_third_person_character))

(fn `UserConstructionScript`)