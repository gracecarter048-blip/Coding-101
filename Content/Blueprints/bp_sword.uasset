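; Sword item that the third-person character can pick up, use and drop.
; On overlap it caches the character and asks it to try picking up the sword; the Pickup event then snaps it to a left-hand finger socket on the mesh.
; Its primary action plays a camera shutter sound and spawns a Bp_ratts actor at the sword's transform.
; Dropping prints a message and destroys the sword.
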(event `self.ReceiveActorBeginOverlap`
  (params (OtherActor :type "Actor Object Reference"))
  (bind _asbp_third_person_character (cast `/Game/ThirdPerson/Blueprints/BP_ThirdPersonCharacter` OtherActor))
  (set `self.As BP Third Person Character` _asbp_third_person_character)
  (`/Game/ThirdPerson/Blueprints/BP_ThirdPersonCharacter.trytopickupITEM` _asbp_third_person_character self))

(event `/Game/Blueprints/BPI_item.pickup`
  (`GameplayStatics.PlaySound2D` "/Engine/VREditor/Sounds/UI/Object_Snaps_To_Another_Actor.Object_Snaps_To_Another_Actor" 1.0 1.0 0.0 null null)
  (`self.K2_AttachToComponent` (`Character.Mesh` (`self.As BP Third Person Character`)) "middle_01_l" "SnapToTarget" "SnapToTarget" "KeepRelative"))

(event `/Game/Blueprints/BPI_item.primary action`
  (`GameplayStatics.PlaySound2D` "/Engine/VREditor/Sounds/UI/Camera_Shutter.Camera_Shutter" 1.0 1.0 0.0 null null)
  (`|SpawnActorFromClass` "/Game/Blueprints/bp_ratts.bp_ratts_C" (`self.GetTransform`) "Undefined" "MultiplyWithRoot" null null))

(event `/Game/Blueprints/BPI_item.drop`
  (`KismetSystemLibrary.PrintText` "the sword has been dropped")
  (`self.K2_DestroyActor`))

(fn `UserConstructionScript`)