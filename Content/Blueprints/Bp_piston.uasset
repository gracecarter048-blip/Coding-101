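; Piston hazard actor that sends the third-person character back to a checkpoint, with a sound, when it overlaps the Rod.
; A timeline starts at BeginPlay from a small random time offset, so instances can run out of step.
; Its track drives the Cylinder's relative height between two limits, and an Impact event plays an attenuated sound at the actor's location.
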(event `self.ReceiveBeginPlay`
  (`|ExecutionSequence`
    (:`then_0`
      (bind (_direction _vertical_piston_location) (`Timeline|Timeline` :`NewTime` (`KismetMathLibrary.RandomFloatInRange` 0.0 0.5) :!via `SetNewTime` :!label _label)
        (:`Update`
          (`SceneComponent.K2_SetRelativeLocation` (`self.Cylinder`) (`KismetMathLibrary.MakeVector` 0.0 0.0 (`KismetMathLibrary.Lerp` 75.0 300.0 _vertical_piston_location)) false false))
        (:`impact`
          (`GameplayStatics.PlaySoundAtLocation` "/Engine/VREditor/Sounds/VR_ungrab_Cue.VR_ungrab_Cue" (`self.K2_GetActorLocation`) (struct) 1.0 1.0 0.0 "/Game/audio/NewSoundAttenuation.NewSoundAttenuation" null null null))))
    (:`then_1`
      (goto _label))))

(event `self.rod.OnComponentBeginOverlap`
  (params (OverlappedComponent :type "PrimitiveComponent Object Reference") (OtherActor :type "Actor Object Reference") (OtherComp :type "PrimitiveComponent Object Reference") (OtherBodyIndex :type Integer) (bFromSweep :type Boolean) (SweepResult :type "HitResult Structure (by ref)"))
  (bind _asbp_third_person_character (cast `/Game/ThirdPerson/Blueprints/BP_ThirdPersonCharacter` OtherActor))
  (`GameplayStatics.PlaySound2D` "/Engine/VREditor/Sounds/VR_close_Cue.VR_close_Cue" 1.0 1.0 0.0 null null)
  (`/Game/ThirdPerson/Blueprints/BP_ThirdPersonCharacter.reset to check point` _asbp_third_person_character))

(fn `UserConstructionScript`)